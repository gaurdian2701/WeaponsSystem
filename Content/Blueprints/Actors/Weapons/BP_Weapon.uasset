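; BP_Weapon is a weapon actor that drives recoil on the player character's animation.
; InitWeapon stores the owner and caches the ABP_PlayerCharacter anim instance from the owning BP_PlayerCharacter's skeletal mesh.
; DoRecoil prints its inputs, then writes the negated recoil angle and kickback strength into that Animation Blueprint.
; GetWeaponMesh exposes the weapon's static mesh.
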(event EventDoRecoil
  (params (RecoilAngle :type Float%20%28single-precision%29) (KickbackStrength :type Float%20%28single-precision%29))
  (bind _player_abp (Variables|Default|GetPlayer%20ABP))
  (Development|PrintString (Utilities|String|ToString(Text) (Utilities|Text|FormatText "Recoil Angle: {Recoil Angle} 
Kickback Strength : {Kickback Strength}" RecoilAngle KickbackStrength)))
  (Variables|/Game/Blueprints/Anim_Blueprints/ABP_PlayerCharacter.ABP_PlayerCharacter_C|SetCurrent%20Kickback%20Strength _player_abp (* KickbackStrength -1.0))
  (Variables|/Game/Blueprints/Anim_Blueprints/ABP_PlayerCharacter.ABP_PlayerCharacter_C|SetCurrent%20Recoil%20Angle _player_abp (* RecoilAngle -1.0)))

(event EventInitWeapon
  (params (Parent :type Actor%20Object%20Reference))
  (bind _output_get (Variables|Default|SetWeaponOwner Parent))
  (bind _asbp_player_character (Utilities|Casting|CastToBP_PlayerCharacter _output_get))
  (bind _newparam (Default|GetCharacterSkeletalMesh _asbp_player_character))
  (bind _asabp_player_character (Utilities|Casting|CastToABP_PlayerCharacter (Components|SkeletalMesh|GetAnimInstance _newparam)))
  (Variables|Default|SetPlayer%20ABP _asabp_player_character))

(fn ConstructionScript)

(fn GetWeaponMesh
  (return (Variables|Default|GetWeaponStaticMesh)))