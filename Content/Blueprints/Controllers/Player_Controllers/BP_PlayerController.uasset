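; BP_PlayerController is the player controller that routes Enhanced Input to the possessed BP_PlayerCharacter.
; On BeginPlay it adds the IMC_Grounded mapping context to the local player input subsystem.
; On possess it caches the pawn as PlayerPossessed, printing an error if the cast fails.
; Move, Look and Fire actions call the matching character functions, leaving their implementation to the character.
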(event Input|EnhancedActionEvents|EnhancedInputActionIA_Move
  (params (ActionValue :type Vector%202D%20Structure) (ElapsedSeconds :type Float%20%28double-precision%29) (TriggeredSeconds :type Float%20%28double-precision%29) (InputAction :type Input%20Action%20Object%20Reference :default "/Game/Blueprints/Input/IA_Move.IA_Move"))
  (Default|Move (Variables|Default|GetPlayerPossessed) (Math|Conversions|ToVector(Vector2D) ActionValue)))

(event Input|EnhancedActionEvents|EnhancedInputActionIA_Look
  (params (ActionValue :type Vector%202D%20Structure) (ElapsedSeconds :type Float%20%28double-precision%29) (TriggeredSeconds :type Float%20%28double-precision%29) (InputAction :type Input%20Action%20Object%20Reference :default "/Game/Blueprints/Input/IA_Look.IA_Look"))
  (Default|LookAround (Variables|Default|GetPlayerPossessed) (Math|Conversions|ToVector(Vector2D) ActionValue)))

(event Input|EnhancedActionEvents|EnhancedInputActionIA_Fire
  (params (ActionValue :type Boolean) (ElapsedSeconds :type Float%20%28double-precision%29) (TriggeredSeconds :type Float%20%28double-precision%29) (InputAction :type Input%20Action%20Object%20Reference :default "/Game/Blueprints/Input/IA_Fire.IA_Fire"))
  (Class|Fireable|Fire (Variables|Default|GetPlayerPossessed)))

(event EventBeginPlay
  (bind _returnvalue (PlayerController|LocalPlayerSubsystems|GetEnhancedInputLocalPlayerSubsystem))
  (if (Utilities|IsValid _returnvalue)
    (Input|AddMappingContext _returnvalue "/Game/Blueprints/Input/IMC_Grounded.IMC_Grounded" 0 "(bIgnoreAllPressedKeysUntilRelease=True,bForceImmediately=False,bNotifyUserSettings=False)")))

(event EventPossess
  (params (PossessedPawn :type Pawn%20Object%20Reference))
  (bind _asbp_player_character (Utilities|Casting|CastToBP_PlayerCharacter PossessedPawn)
    (:then
      (Variables|Default|SetPlayerPossessed _asbp_player_character))
    (:CastFailed
      (Development|PrintString "CAST FAILURE! PLEASE SUPPLY CORRECT PLAYER CLASS OR CHANGE THE PLAYER CLASS " true true "(R=0.494792,G=0.000000,B=0.042046,A=1.000000)"))))

(fn ConstructionScript)