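; Player character Blueprint that handles movement, looking and use of an equipped weapon.
; Move and LookAround turn 2D input into actor-relative movement and controller yaw and pitch.
; EquipWeapon casts to BP_Weapon, stores it and initializes it with the character as owner, and Fire forwards to that weapon.
; Getters expose the skeletal mesh and a firing start position, which is only a zero-vector placeholder.
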(event EventFire
  (Class|Fireable|Fire (Variables|Default|GetEquippedWeapon)))

(event EventEquipWeapon
  (params (Weapon :type Weapon%20Object%20Reference))
  (bind _asbp_weapon (Utilities|Casting|CastToBP_Weapon Weapon))
  (bind _output_get (Variables|Default|SetEquippedWeapon _asbp_weapon))
  (Class|Weapon|InitWeapon _output_get self))

(fn ConstructionScript)

(fn Move
  (params (NewParam :type Vector))
  (Pawn|Input|AddMovementInput (* (.y NewParam) (Transformation|GetActorForwardVector)) 1.0 false)
  (Pawn|Input|AddMovementInput (* (.x NewParam) (Transformation|GetActorRightVector)) 1.0 false))

(fn LookAround
  (params (NewParam :type Vector))
  (Pawn|Input|AddControllerYawInput (.x NewParam))
  (bind _result (Math|Float|NegateFloat (.y NewParam))
    (:%20%20
      (Pawn|Input|AddControllerPitchInput _result))))

(fn GetCharacterSkeletalMesh
  (return (Variables|Default|GetSkeletalMesh)))

(fn GetFiringStartPosition
  (return "0, 0, 0"))